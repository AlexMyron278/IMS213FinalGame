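; BP_Door is a level-exit door that sends the third-person character to the End_Screen level once they have collected at least ten coal.
; On overlap it casts to BP_ThirdPersonCharacter and checks CoalCount.
; When coal is short, it shows a Popup_Text widget for a few seconds, creating it on first contact and toggling the cached instance's visibility afterward.
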(event `self.ReceiveActorBeginOverlap`
  (params (OtherActor :type "Actor Object Reference"))
  (bind _popup_text (`self.Popup_Text`))
  (bind _asbp_third_person_character (cast `/Game/ThirdPerson/Blueprints/BP_ThirdPersonCharacter` OtherActor))
  (if (<= 10 (`/Game/ThirdPerson/Blueprints/BP_ThirdPersonCharacter.Coal_Count` _asbp_third_person_character))
    (`GameplayStatics.OpenLevelBySoftObjectPtr` "/Game/MyMaps/End_Screen.End_Screen")
    (elif (`self.Popup_Made`)
      (`Widget.SetVisibility` _popup_text "Visible")
      (`KismetSystemLibrary.Delay` 3.0)
      (`Widget.SetVisibility` _popup_text "Hidden")
      (else
        (bind _returnvalue (`|CreateWidget` "/Game/Blueprints/Popup_Text.Popup_Text_C"))
        (set `self.Popup_Text` _returnvalue)
        (set `self.Popup_Made` true)
        (`UserWidget.AddToViewport` _returnvalue 0)
        (`KismetSystemLibrary.Delay` 2.0)
        (`Widget.SetVisibility` _returnvalue "Hidden")))))

(fn `UserConstructionScript`)